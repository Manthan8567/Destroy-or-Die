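; Damagable object Blueprint that can bob on the Z axis and shatters with Chaos destruction when its health runs out.
; A looping timeline drives the bobbing, started after a random delay.
; AnyDamage reduces health only for damage types listed in DamagableBy.
; Breaking swaps the static mesh for a geometry collection, applies strain and radial force, plays a sound, fires OnBreak and destroys the actor after a delay.
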(event `self.ReceiveBeginPlay`
  (`KismetSystemLibrary.Delay` (`KismetMathLibrary.RandomFloat`))
  (set `self.InitialActorLocation` (`self.K2_GetActorLocation`))
  (`self.MoveUpAndDown`))

(event `MoveUpAndDown`
  (bind (_initialactorlocation_x _initialactorlocation_y _initialactorlocation_z) (`KismetMathLibrary.BreakVector` (`self.InitialActorLocation`)))
  (bind (_actorlocationbeforemoving_x _actorlocationbeforemoving_y _actorlocationbeforemoving_z) (`KismetMathLibrary.BreakVector` (`self.ActorLocationBeforeMoving`)))
  (if (`self.ShouldMove`)
    (`self.StaticMesh`
      (:`then`
        (set `self.ActorLocationBeforeMoving` (`self.K2_GetActorLocation`))
        (bind (_direction _movezalpha) (`Timeline|MoveTimeline` :!via `PlayFromStart` :!label _label)
          (:`Update`
            (`self.K2_SetActorLocation` (`KismetMathLibrary.MakeVector` _actorlocationbeforemoving_x _actorlocationbeforemoving_y (`KismetMathLibrary.Lerp` _actorlocationbeforemoving_z (+ _initialactorlocation_z (`self.MaxMoveOnZAxis`)) _movezalpha))))
          (:`Finished`
            (`self.MoveUpAndDown`))))
      (:`else`))))

(event `StopMovingUpAndDown`
  (goto _label :!via `Stop`))

(event `self.ReceiveAnyDamage`
  (params (Damage :type "Float (single-precision)") (DamageType :type "DamageType Object Reference") (InstigatedBy :type "Controller Object Reference") (DamageCauser :type "Actor Object Reference"))
  (if (`KismetArrayLibrary.Array_Contains` (`self.DamagableBy`) (`GameplayStatics.GetObjectClass` DamageType))
    (bind _output_get (set `self.Health` (`KismetMathLibrary.FClamp` (- (`self.Health`) Damage) 0.0 (`self.MaxHealth`))))
    (if (<= _output_get 0.0)
      (`/Engine/EditorBlueprintResources/StandardMacros.DoOnce` false
        (:`Completed`
          (`self.Break`))))))

(event `AddFracturedGeometry`
  (bind _returnvalue (`AddComponent|NODE_AddGeometryCollectionComponent-1`))
  (set `self.FracturedGeometryCollection` _returnvalue))

(event `Break`
  (`ActorComponent.K2_DestroyComponent` (`self.StaticMesh`))
  (set `self.ShouldMove` false)
  (`self.AddFracturedGeometry`)
  (`FieldSystemComponent.ApplyPhysicsField` (`self.FieldSystem`) true "Field_ExternalClusterStrain" null (`RadialFalloff.SetRadialFalloff` (`self.RadialFalloff`) 100.0 0.0 1.0 0.0 100.0 (`self.K2_GetActorLocation`) "Field_FallOff_None"))
  (`ActorComponent.Activate` (`self.RadialForce`) false)
  (`GameplayStatics.PlaySoundAtLocation` (`self.BreakingSound`) (`self.K2_GetActorLocation`) (struct) 1.0 1.0 0.0 null null null null)
  (`self.OnBreak` self)
  (`KismetSystemLibrary.Delay` 3.0)
  (`self.K2_DestroyActor`))

(fn `UserConstructionScript`)