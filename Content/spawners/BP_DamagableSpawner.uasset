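; A spawner actor that places damageable ranged or melee targets at random points inside a box volume.
; The construction script sizes the box from an Area variable, and SpawnRandomDamagable picks one of the two target types at random.
; Ranged targets get a random height between MinZ and MaxZ and are rotated to face the player character, while melee targets spawn at a fixed default height.
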(fn `SpawnMeleeDamagable`
  (params (Location :type "Vector Structure"))
  (returns (MeleeDamagable :type "/Game/Damagable/BP_DamagableObject_MeleeTarget Object Reference"))
  (locals (DefaultZLocation :type "Float (double-precision)" :default 157.0))
  (bind _returnvalue (`|SpawnActorFromClass` "/Game/Damagable/BP_DamagableObject_MeleeTarget.BP_DamagableObject_MeleeTarget_C" (`KismetMathLibrary.MakeTransform` (`KismetMathLibrary.MakeVector` Location_X Location_Y (`local.DefaultZLocation`))) "Undefined" "MultiplyWithRoot" null null))
  (return _returnvalue))

(fn `SpawnRandomDamagable`
  (returns (DamagableObject :type "/Game/Damagable/BP_DamagableObject Object Reference"))
  (bind (_origin _boxextent) (`KismetSystemLibrary.GetComponentBounds` (`self.Box`)))
  (bind _returnvalue (`KismetMathLibrary.RandomPointInBoundingBox` _origin _boxextent))
  (switch `int` (`KismetMathLibrary.RandomInteger` 2)
    (:`0`
      (bind _rangeddamagable (`self.SpawnRangedDamagable` _returnvalue))
      (return _rangeddamagable))
    (:`1`
      (bind _meleedamagable (`self.SpawnMeleeDamagable` _returnvalue))
      (return _meleedamagable))))

(fn `SpawnRangedDamagable`
  (params (Location :type "Vector Structure"))
  (returns (RangedDamagable :type "/Game/Damagable/BP_DamagableObject_RangedTarget Object Reference"))
  (locals (MinZ :type "Float (double-precision)" :default 350.0) (MaxZ :type "Float (double-precision)" :default 600.0))
  (bind _returnvalue (`|SpawnActorFromClass` "/Game/Damagable/BP_DamagableObject_RangedTarget.BP_DamagableObject_RangedTarget_C" (`KismetMathLibrary.MakeTransform` (`KismetMathLibrary.MakeVector` Location_X Location_Y (`KismetMathLibrary.RandomFloatInRange` (`local.MinZ`) (`local.MaxZ`)))) "Undefined" "MultiplyWithRoot" null null))
  (`self.K2_SetActorRotation` _returnvalue (`KismetMathLibrary.FindLookAtRotation` (`self.K2_GetActorLocation` _returnvalue) (`self.K2_GetActorLocation` (`GameplayStatics.GetPlayerCharacter` 0))) false)
  (return _returnvalue))

(fn `UserConstructionScript`
  (`BoxComponent.SetBoxExtent` (`self.Box`) (`self.Area`) true))