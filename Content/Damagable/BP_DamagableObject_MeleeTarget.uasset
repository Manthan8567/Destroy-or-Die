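; BP_DamagableObject_MeleeTarget is a damageable target that spins on Z and reacts to melee hits.
; A self-restarting timeline drives continuous yaw rotation from BeginPlay.
; DT_Melee damage briefly halts rotation and up-and-down movement while boosting emissive glow on a dynamic material created in construction, then resumes both.
; It supplies its own geometry collection component through AddFracturedGeometry and relies on its parent for general damage handling.
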(event `self.ReceiveBeginPlay`
  (`parent.ReceiveBeginPlay`)
  (`self.RotateOnZ`))

(event `self.AddFracturedGeometry`
  (bind _returnvalue (`AddComponent|NODE_AddGeometryCollectionComponent-0`))
  (set `self.FracturedGeometryCollection` _returnvalue))

(event `RotateOnZ`
  (bind (_rotationbeforerotating_roll _rotationbeforerotating_pitch _rotationbeforerotating_yaw) (`KismetMathLibrary.BreakRotator` (`self.RotationBeforeRotating`)))
  (set `self.RotationBeforeRotating` (`self.K2_GetActorRotation`))
  (bind (_direction _zalpha) (`Timeline|RotateTimeline` :!via `PlayFromStart` :!label _label)
    (:`Update`
      (`self.K2_SetActorRotation` (`KismetMathLibrary.MakeRotator` 0.0 0.0 (`KismetMathLibrary.Lerp` _rotationbeforerotating_yaw (+ _rotationbeforerotating_yaw 360.0) _zalpha))))
    (:`Finished`
      (`self.RotateOnZ`))))

(event `StopRotatingOnZ`
  (goto _label :!via `Stop`))

(event `self.ReceiveAnyDamage`
  (params (Damage :type "Float (single-precision)") (DamageType :type "DamageType Object Reference") (InstigatedBy :type "Controller Object Reference") (DamageCauser :type "Actor Object Reference"))
  (`parent.ReceiveAnyDamage` Damage DamageType InstigatedBy DamageCauser)
  (if (== (`GameplayStatics.GetObjectClass` DamageType) "/Game/Damagable/DT_Melee.DT_Melee_C")
    (`self.StopMovingUpAndDown`)
    (`self.StopRotatingOnZ`)
    (`MaterialInstanceDynamic.SetScalarParameterValue` (`self.MeshDynamicMaterial`) "Emissive color 01 multiply" 20.0)
    (`KismetSystemLibrary.Delay` 0.3)
    (`self.MoveUpAndDown`)
    (`self.RotateOnZ`)
    (`MaterialInstanceDynamic.SetScalarParameterValue` (`self.MeshDynamicMaterial`) "Emissive color 01 multiply" 1.0)))

(fn `UserConstructionScript`
  (`parent.UserConstructionScript`)
  (bind _returnvalue (`KismetMaterialLibrary.CreateDynamicMaterialInstance` "/Game/StarterContent/Materials/M_Tech_Hex_Tile_Pulse_Inst.M_Tech_Hex_Tile_Pulse_Inst"))
  (bind _output_get (set `self.MeshDynamicMaterial` _returnvalue))
  (`PrimitiveComponent.SetMaterial` (`self.StaticMesh`) 0 _output_get))